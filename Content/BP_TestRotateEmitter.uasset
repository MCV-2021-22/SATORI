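; BP_TestRotateEmitter is a test actor that orbits the point where it starts play, facing that center.
; BeginPlay stores the starting location as Center, and Tick advances an angle by RotationSpeed, resetting it to zero at a full turn.
; Tick rotates the RelativeLocation offset around AxisVector, adds it to Center, and sets location with a look-at rotation computed from the pre-move position.
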(event EventBeginPlay
  (Variables|Default|SetCenter (Transformation|GetActorLocation)))

(event EventTick
  (params (DeltaSeconds :type Float%20%28single-precision%29))
  (Variables|Default|SetNewLocation (Variables|Default|GetCenter))
  (bind _output_get (Variables|Default|SetAngleAxis (+ (Variables|Default|GetAngleAxis) (* DeltaSeconds (Variables|Default|GetRotationSpeed)))))
  (if (>= _output_get 3.6e+02)
    (bind _output_get_2 (Variables|Default|SetAngleAxis 0.0)))
  (bind _output_get_3 (Variables|Default|SetNewRotation (Math|Vector|RotateVectorAroundAxis (Variables|Default|GetRelativeLocation) _output_get_2 (Variables|Default|GetAxisVector))))
  (Transformation|SetActorLocationAndRotation (Math|Vector|MakeVector (+ (.x (Variables|Default|GetNewLocation)) (.x _output_get_3)) (+ (.y _output_get_3) (.y (Variables|Default|GetNewLocation))) (+ (.z _output_get_3) (.z (Variables|Default|GetNewLocation)))) (Math|Rotator|FindLookatRotation (Transformation|GetActorLocation) (Variables|Default|GetCenter))))

(fn ConstructionScript)