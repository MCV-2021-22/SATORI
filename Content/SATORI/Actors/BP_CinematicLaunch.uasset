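; Trigger actor that launches a cinematic when the SATORI character overlaps its Box.
; The overlap disables the character's input, then plays the first LevelSequenceActor found in the level via GetActorOfClass.
; A fixed delay, not tied to the sequence's end, restores input and destroys the trigger.
; If no sequence actor is found, input stays disabled.
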(event OnComponentBeginOverlap(Box)
  (params (OverlappedComponent :type Primitive%20Component%20Object%20Reference) (OtherActor :type Actor%20Object%20Reference) (OtherComp :type Primitive%20Component%20Object%20Reference) (OtherBodyIndex :type Integer) (bFromSweep :type Boolean) (SweepResult :type Hit%20Result%20Structure%20%28by%20ref%29))
  (bind _assatori_character (Utilities|Casting|CastToSATORI_Character OtherActor))
  (Input|DisableInput _assatori_character (Game|GetPlayerController 0))
  (bind _returnvalue (Actor|GetActorOfClass "/Script/LevelSequence.LevelSequenceActor"))
  (Utilities|IsValid _returnvalue
    (:Is%20Valid
      (Sequencer|Player|Play (Variables|/Script/LevelSequence.LevelSequenceActor|GetSequencePlayer _returnvalue) :!class /Script/MovieScene.MovieSceneSequencePlayer)
      (Utilities|FlowControl|Delay 1e+01)
      (Input|EnableInput _assatori_character (Game|GetPlayerController 0))
      (Actor|DestroyActor))))

(event EventBeginPlay)

(event Collision|EventActorBeginOverlap
  (params (OtherActor :type Actor%20Object%20Reference)))

(event EventTick
  (params (DeltaSeconds :type Float%20%28single-precision%29)))

(fn ConstructionScript)