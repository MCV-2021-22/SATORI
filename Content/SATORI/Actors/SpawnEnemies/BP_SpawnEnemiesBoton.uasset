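; Button actor that brings the game mode's enemies into play, showing its widget while something overlaps its box.
; Its SpawnEnemies event hides the widget and loops over the SATORI game mode's enemy references, moving each valid AI character to its desired Z height and activating its movement.
; Within that loop it starts a timeline that sinks the button into a lower position, then destroys it.
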(event OnComponentBeginOverlap(Box)
  (params (OverlappedComponent :type Primitive%20Component%20Object%20Reference) (OtherActor :type Actor%20Object%20Reference) (OtherComp :type Primitive%20Component%20Object%20Reference) (OtherBodyIndex :type Integer) (bFromSweep :type Boolean) (SweepResult :type Hit%20Result%20Structure%20%28by%20ref%29))
  (Rendering|SetVisibility (Variables|Default|GetWidget) true false))

(event OnComponentEndOverlap(Box)
  (params (OverlappedComponent :type Primitive%20Component%20Object%20Reference) (OtherActor :type Actor%20Object%20Reference) (OtherComp :type Primitive%20Component%20Object%20Reference) (OtherBodyIndex :type Integer))
  (Rendering|SetVisibility (Variables|Default|GetWidget) false false))

(event Custom|Spawn%20Enemies
  (Variables|Default|SetLocation (Transformation|GetActorLocation self))
  (Rendering|SetVisibility (Variables|Default|GetWidget) false false)
  (bind _assatorigame_mode (Utilities|Casting|CastToSATORIGameMode (Game|GetGameMode)))
  (bind _returnvalue (Class|SATORIGameMode|GetEnemyActorsRef _assatorigame_mode))
  (for _array_element _returnvalue
    (Utilities|IsValid _array_element
      (:Is%20Valid
        (bind _assatori_aicharacter (Utilities|Casting|CastToSATORI_AICharacter _array_element))
        (Transformation|SetActorLocation _assatori_aicharacter (Math|Vector|MakeVector (.X (Math|Vector|BreakVector (Transformation|GetActorLocation _assatori_aicharacter))) (.Y (Math|Vector|BreakVector (Transformation|GetActorLocation _assatori_aicharacter))) (Variables|/Script/SATORI.SATORI_AICharacter|GetDesiredZPosition _assatori_aicharacter)) false false)
        (Components|Activation|Activate (Variables|/Script/Engine.Character|GetCharacterMovement _assatori_aicharacter) false)
        (bind _newtrack_0 (Timeline|Timeline_0 Play)
          (:Update
            (Transformation|SetActorLocation (Math|Vector|Lerp(Vector) (Variables|Default|GetLocation) (- (Variables|Default|GetLocation) "0, 0,200.000000") _newtrack_0) false false))
          (:Finished
            (Actor|DestroyActor)))))))

(fn ConstructionScript)