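; BP_SpawnEnemiesTrigger is a trigger box that brings tagged AI enemies into play when a SATORI_Character overlaps it.
; It finds every actor tagged PossessedBy.AI, moves each SATORI_AICharacter to its DesiredZPosition while keeping X and Y, and activates its movement component.
; Enemies are repositioned rather than spawned, and the trigger calls DestroyActor on itself from inside the loop.
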(event OnComponentBeginOverlap(Box)
  (params (OverlappedComponent :type Primitive%20Component%20Object%20Reference) (OtherActor :type Actor%20Object%20Reference) (OtherComp :type Primitive%20Component%20Object%20Reference) (OtherBodyIndex :type Integer) (bFromSweep :type Boolean) (SweepResult :type Hit%20Result%20Structure%20%28by%20ref%29))
  (Utilities|Casting|CastToSATORI_Character OtherActor)
  (bind _outactors (Actor|GetAllActorswithTag "PossessedBy.AI"))
  (for _array_element _outactors
    (bind _assatori_aicharacter (Utilities|Casting|CastToSATORI_AICharacter _array_element))
    (Transformation|SetActorLocation _assatori_aicharacter (Math|Vector|MakeVector (.X (Math|Vector|BreakVector (Transformation|GetActorLocation _assatori_aicharacter))) (.Y (Math|Vector|BreakVector (Transformation|GetActorLocation _assatori_aicharacter))) (Variables|/Script/SATORI.SATORI_AICharacter|GetDesiredZPosition _assatori_aicharacter)) false false)
    (Components|Activation|Activate (Variables|/Script/Engine.Character|GetCharacterMovement _assatori_aicharacter) false)
    (Actor|DestroyActor)))

(event EventBeginPlay)

(event Collision|EventActorBeginOverlap
  (params (OtherActor :type Actor%20Object%20Reference)))

(event EventTick
  (params (DeltaSeconds :type Float%20%28single-precision%29)))

(fn ConstructionScript)