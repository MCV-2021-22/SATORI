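; BP_Farolillo is a self-destroying lantern actor whose static mesh moves vertically along a timeline.
; BeginPlay starts the timeline, which sets the mesh's relative Z from the track's Z value while keeping X and Y.
; Whenever that value is exactly zero, a random vertical offset is added for that update only; later non-zero values overwrite it.
; The actor destroys itself when the timeline finishes.
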(event EventBeginPlay
  (bind _staticmesh (Variables|Default|GetStaticMesh))
  (bind _relativelocation (Variables|/Script/Engine.SceneComponent|GetRelativeLocation _staticmesh))
  (bind _newtrack_0 (Timeline|Timeline_0 Play)
    (:Update
      (if (== (.Z (Math|Vector|BreakVector _newtrack_0)) 0.0)
        (Transformation|SetRelativeLocation (Variables|Default|GetStaticMesh) (Math|Vector|MakeVector (.x _relativelocation) (.y _relativelocation) (+ (.Z (Math|Vector|BreakVector _newtrack_0)) (Math|Random|RandomFloatinRange -1e+03 1e+03))) false false)
        (else
          (Transformation|SetRelativeLocation (Variables|Default|GetStaticMesh) (Math|Vector|MakeVector (.x _relativelocation) (.y _relativelocation) (.Z (Math|Vector|BreakVector _newtrack_0))) false false))))
    (:Finished
      (Actor|DestroyActor))))

(event Collision|EventActorBeginOverlap
  (params (OtherActor :type Actor%20Object%20Reference)))

(fn ConstructionScript)