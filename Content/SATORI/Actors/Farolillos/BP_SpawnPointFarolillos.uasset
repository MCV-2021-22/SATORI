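; BP_SpawnPointFarolillos is a spawner actor that periodically fills a volume with batches of BP_Farolillo actors.
; From BeginPlay it spawns a batch, waits a random few seconds, then repeats indefinitely through a looping retriggerable delay.
; Each actor appears at a random point within the Bound component's box, adjusted for collision but always spawned.
; Yaw uses an unscaled RandomFloat, so rotation varies by at most one degree.
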(event Custom|Spawn%20Character
  (bind _bound (Variables|Default|GetBound))
  (bind (_origin _boxextent) (Collision|GetComponentBounds _bound))
  (for _index (range 0 20)
    (Game|SpawnActorfromClass "/Game/SATORI/Actors/Farolillos/BP_Farolillo.BP_Farolillo_C" (Math|Transform|MakeTransform (Math|Random|RandomPointinBoundingBox _origin _boxextent) (Math|Rotator|MakeRotator 0.0 0.0 (Math|Random|RandomFloat))) "AdjustIfPossibleButAlwaysSpawn" 0 0)))

(event EventBeginPlay
  (CallFunction|SpawnCharacter :!label _label)
  (Utilities|FlowControl|RetriggerableDelay (Math|Random|RandomFloatinRange 5.0 1e+01))
  (goto _label))

(fn ConstructionScript)