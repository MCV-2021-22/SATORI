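; Pull ability actor that draws a Niagara beam from the player character's hand to an AI character it overlaps.
; On BeginPlay it attaches the beam effect to the hand and deactivates it after a short delay.
; The collision sphere records the overlapped AI, and Tick moves the beam end to that target.
; Once the target is close to the player, a flag clears and the actor destroys itself on a later tick.
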(event OnComponentBeginOverlap(CollisionSphereComponent)
  (params (OverlappedComponent :type Primitive%20Component%20Object%20Reference) (OtherActor :type Actor%20Object%20Reference) (OtherComp :type Primitive%20Component%20Object%20Reference) (OtherBodyIndex :type Integer) (bFromSweep :type Boolean) (SweepResult :type Hit%20Result%20Structure%20%28by%20ref%29))
  (bind _assatori_aicharacter (Utilities|Casting|CastToSATORI_AICharacter OtherActor))
  (Variables|Default|SetPullingChar _assatori_aicharacter))

(event EventBeginPlay
  (bind _assatori_character (Utilities|Casting|CastToSATORI_Character (Game|GetPlayerCharacter 0)))
  (Variables|Default|SetAs%20SATORI%20Character _assatori_character)
  (bind _returnvalue (Niagara|SpawnSystemAttached "/Game/SATORI/Actors/Pull/NS_Pull.NS_Pull" (Variables|/Script/SATORI.SATORICharacter|GetHandComponent _assatori_character) "None" (Transformation|GetWorldLocation (Variables|/Script/SATORI.SATORICharacter|GetHandComponent _assatori_character)) "0, 0, 0" "KeepWorldPosition" false))
  (Variables|Default|SetNiagara _returnvalue)
  (Utilities|FlowControl|Delay 3.0)
  (Components|Activation|Deactivate (Variables|Default|GetNiagara)))

(event EventTick
  (params (DeltaSeconds :type Float%20%28single-precision%29))
  (bind _pullingchar (Variables|Default|GetPullingChar))
  (bind _returnvalue (Transformation|GetActorLocation _pullingchar))
  (if (Variables|Default|GetCondition)
    (Utilities|IsValid _pullingchar
      (:Is%20Valid
        (Effects|Components|ParticleSystem|SetVectorParameter (Variables|Default|GetNiagara) "User.Beam End" _returnvalue)
        (if (< (Math|Vector|Distance(Vector) _returnvalue (Transformation|GetActorLocation (Variables|Default|GetAs%20SATORI%20Character))) 1.5e+02)
          (Variables|Default|SetCondition false))))
    (else
      (Components|Activation|Deactivate (Variables|Default|GetNiagara))
      (Actor|DestroyActor))))

(fn ConstructionScript)