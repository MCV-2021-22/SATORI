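; Spawner enemy Blueprint that handles cosmetic physics, targeting registration and damage feedback; no spawning of enemies happens in this graph.
; On BeginPlay it simulates physics on two rope bone chains, registers as targetable and caches max health.
; Tick projects the health bar, then, as does the stat component's health event, refreshes it and accumulates health changes.
; A retriggerable delay merges rapid hits into one floating damage number.
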(event UpdateHealthBarPercent(EnemyStatComponent)
  (params (Health :type Float%20%28single-precision%29) (MaxHealth :type Float%20%28single-precision%29))
  ;[1 1 1] Update UI Tick
  (bind _aswp_enemy_life_bar (Utilities|Casting|CastToWP_EnemyLifeBar (UserInterface|GetWidget (Variables|Default|GetHealthBar))))
  (Class|SATORIEnemyHealthBar|UpdateHealthBar _aswp_enemy_life_bar Health MaxHealth)
  (if (!= Health (Variables|Default|GetOldHealth))
    (Variables|Default|SetStackDamage (+ (Variables|Default|GetStackDamage) (- (Variables|Default|GetOldHealth) Health)))
    (Variables|Default|SetOldHealth Health)
    (Utilities|FlowControl|RetriggerableDelay 0.5)
    (if (> (Variables|Default|GetStackDamage) 0.0)
      (Game|SpawnActorfromClass "/Game/SATORI/UI/Player/BP_DamageNumber.BP_DamageNumber_C" (Math|Transform|MakeTransform (Transformation|GetActorLocation) "0, 0, 0" "1,1,1") "Undefined" 0 (Math|Float|Truncate (Variables|Default|GetStackDamage)) 0)
      (Variables|Default|SetStackDamage 0.0))))

(event Collision|EventActorBeginOverlap
  (params (OtherActor :type Actor%20Object%20Reference)))

(event EventTick
  (params (DeltaSeconds :type Float%20%28single-precision%29))
  (bind _healthbar (Variables|Default|GetHealthBar))
  ;[1 1 1] Update UI Tick
  (Class|SATORIAICharacter|HealthBarProjection _healthbar 2048.0 0.1 0.5)
  (bind _aswp_enemy_life_bar (Utilities|Casting|CastToWP_EnemyLifeBar (UserInterface|GetWidget _healthbar)))
  (Class|SATORIEnemyHealthBar|UpdateHealthBar _aswp_enemy_life_bar (stale UpdateHealthBarPercent(EnemyStatComponent) Health) (stale UpdateHealthBarPercent(EnemyStatComponent) MaxHealth))
  (if (!= (stale UpdateHealthBarPercent(EnemyStatComponent) Health) (Variables|Default|GetOldHealth))
    (Variables|Default|SetStackDamage (+ (Variables|Default|GetStackDamage) (- (Variables|Default|GetOldHealth) (stale UpdateHealthBarPercent(EnemyStatComponent) Health))))
    (Variables|Default|SetOldHealth (stale UpdateHealthBarPercent(EnemyStatComponent) Health))
    (Utilities|FlowControl|RetriggerableDelay 0.5)
    (if (> (Variables|Default|GetStackDamage) 0.0)
      (Game|SpawnActorfromClass "/Game/SATORI/UI/Player/BP_DamageNumber.BP_DamageNumber_C" (Math|Transform|MakeTransform (Transformation|GetActorLocation) "0, 0, 0" "1,1,1") "Undefined" 0 (Math|Float|Truncate (Variables|Default|GetStackDamage)) 0)
      (Variables|Default|SetStackDamage 0.0))))

(event EventBeginPlay
  (Utilities|FlowControl|Sequence
    (:then_0
      (Class|SkeletalMeshComponent|SetAllBodiesBelowSimulatePhysics (Variables|Character|GetMesh) (Utilities|Name|MakeLiteralName "Bip001-Rope_1") true true)
      (Class|SkeletalMeshComponent|SetAllBodiesBelowSimulatePhysics (Variables|Character|GetMesh) (Utilities|Name|MakeLiteralName "Bip001-Rope_2") true true))
    (:then_1
      (Class|SATORIAICharacter|RegisterinTargetableArray)
      (Variables|Default|SetOldHealth (Class|SATORICharacterBase|GetMaxHealth)))))

(fn ConstructionScript)