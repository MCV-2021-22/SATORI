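; Fujin boss enemy Blueprint that registers itself with the player character's boss arrow on BeginPlay and drives its own health bar.
; Tick runs the health bar projection on the widget component, then pushes Health and MaxHealth into the WP_EnemyLifeBar widget.
; The stat component's UpdateHealthBarPercent event feeds the same widget update.
; The cloud particle spawn and socket attachment nodes are disconnected and never run.
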(event UpdateHealthBarPercent(EnemyStatComponent)
  (params (Health :type Float%20%28single-precision%29) (MaxHealth :type Float%20%28single-precision%29))
  (bind _aswp_enemy_life_bar (Utilities|Casting|CastToWP_EnemyLifeBar (UserInterface|GetWidget (Variables|Default|GetHealthWidget))))
  (Class|SATORIEnemyHealthBar|UpdateHealthBar _aswp_enemy_life_bar Health MaxHealth))

(event EventBeginPlay
  (bind _assatori_character (Utilities|Casting|CastToSATORI_Character (Game|GetPlayerCharacter 0)))
  (Default|BossArrow _assatori_character self))

(event Collision|EventActorBeginOverlap
  (params (OtherActor :type Actor%20Object%20Reference)))

(event EventTick
  (params (DeltaSeconds :type Float%20%28single-precision%29))
  (bind _healthwidget (Variables|Default|GetHealthWidget))
  (Class|SATORIAICharacter|HealthBarProjection _healthwidget 2048.0 0.1 0.5)
  (bind _aswp_enemy_life_bar (Utilities|Casting|CastToWP_EnemyLifeBar (UserInterface|GetWidget _healthwidget)))
  (Class|SATORIEnemyHealthBar|UpdateHealthBar _aswp_enemy_life_bar (stale UpdateHealthBarPercent(EnemyStatComponent) Health) (stale UpdateHealthBarPercent(EnemyStatComponent) MaxHealth)))

(fn ConstructionScript)