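; BP_RangeMovable is a SATORI AI enemy Blueprint that handles targeting registration, health display and damage feedback.
; On BeginPlay it registers as targetable and either initializes the W_Debug widget or destroys that component.
; Tick projects and updates the health bar, polling Health for changes.
; Changes accumulate through a short retriggerable delay, then spawn one BP_DamageNumber with the stacked damage.
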(event UpdateHealthBarPercent(EnemyStatComponent)
  (params (Health :type Float%20%28single-precision%29) (MaxHealth :type Float%20%28single-precision%29))
  ;[1 1 1] Update UI Tick
)

(event Collision|EventActorBeginOverlap
  (params (OtherActor :type Actor%20Object%20Reference)))

(event EventTick
  (params (DeltaSeconds :type Float%20%28single-precision%29))
  (bind _healthwidget (Variables|Default|GetHealthWidget))
  ;[1 1 1] Update UI Tick
  (Class|SATORIAICharacter|HealthBarProjection _healthwidget 2048.0 0.1 0.5)
  (bind _aswp_enemy_life_bar (Utilities|Casting|CastToWP_EnemyLifeBar (UserInterface|GetWidget _healthwidget)))
  (Class|SATORIEnemyHealthBar|UpdateHealthBar _aswp_enemy_life_bar (stale UpdateHealthBarPercent(EnemyStatComponent) Health) (stale UpdateHealthBarPercent(EnemyStatComponent) MaxHealth))
  (if (!= (stale UpdateHealthBarPercent(EnemyStatComponent) Health) (Variables|Default|GetOldHealth))
    (Variables|Default|SetStackDamage (+ (Variables|Default|GetStackDamage) (- (Variables|Default|GetOldHealth) (stale UpdateHealthBarPercent(EnemyStatComponent) Health))))
    (Variables|Default|SetOldHealth (stale UpdateHealthBarPercent(EnemyStatComponent) Health))
    (Utilities|FlowControl|RetriggerableDelay 0.1)
    (if (> (Variables|Default|GetStackDamage) 0.0)
      (Game|SpawnActorfromClass "/Game/SATORI/UI/Player/BP_DamageNumber.BP_DamageNumber_C" (Math|Transform|MakeTransform (Transformation|GetActorLocation) "0, 0, 0" "1,1,1") "Undefined" 0 (Math|Float|Truncate (Variables|Default|GetStackDamage)) 0)
      (Variables|Default|SetStackDamage 0.0))))

(event EventBeginPlay
  (bind _debug (Variables|Default|GetDebug))
  (Class|SATORIAICharacter|RegisterinTargetableArray)
  (if (Variables|Default|GetbShowDebug)
    (bind _asw_debug (Utilities|Casting|CastToW_Debug (UserInterface|GetWidget _debug)))
    (Default|InitCharacter _asw_debug self (Variables|Default|GetAttributes%20to%20Debug) (Variables|Default|GetAbilities%20Cooldown%20Tags))
    (else
      (Components|DestroyComponent _debug))))

(fn ConstructionScript)