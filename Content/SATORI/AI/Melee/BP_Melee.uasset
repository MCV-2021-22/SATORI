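; BP_Melee is a melee AI enemy Blueprint with an overhead health bar and an optional debug display.
; On BeginPlay it enables physics on selected mesh bone chains, switches it back off for specific bones, and either initializes the ability and attribute debug widget or destroys it.
; Tick projects the health bar by view distance and refreshes its values, an update also triggered by the stat component's health event.
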(event UpdateHealthBarPercent(EnemyStatComponent)
  (params (Health :type Float%20%28single-precision%29) (MaxHealth :type Float%20%28single-precision%29))
  ;[1 1 1] Update UI Tick
  (bind _aswp_enemy_life_bar (Utilities|Casting|CastToWP_EnemyLifeBar (UserInterface|GetWidget (Variables|Default|GetHealthWidget))))
  (Class|SATORIEnemyHealthBar|UpdateHealthBar _aswp_enemy_life_bar Health MaxHealth))

(event EventBeginPlay
  (bind _debug (Variables|Default|GetDebug))
  (Utilities|FlowControl|Sequence
    (:then_0
      (Class|SkeletalMeshComponent|SetAllBodiesBelowSimulatePhysics (Variables|Character|GetMesh) (Utilities|Name|MakeLiteralName "Bone023") true true)
      (Class|SkeletalMeshComponent|SetAllBodiesBelowSimulatePhysics (Variables|Character|GetMesh) (Utilities|Name|MakeLiteralName "Bone046") false true)
      (Class|SkeletalMeshComponent|SetAllBodiesBelowSimulatePhysics (Variables|Character|GetMesh) (Utilities|Name|MakeLiteralName "Bone001") true true)
      (Class|SkeletalMeshComponent|SetAllBodiesBelowSimulatePhysics (Variables|Character|GetMesh) (Utilities|Name|MakeLiteralName "Bone021") false true))
    (:then_1
      (if (Variables|Default|GetbShowDebug)
        (bind _asw_debug (Utilities|Casting|CastToW_Debug (UserInterface|GetWidget _debug)))
        (Default|InitCharacter _asw_debug self (Variables|Default|GetAttributes%20to%20Debug) (Variables|Default|GetAbilities%20Cooldown%20Tags))
        (else
          (Components|DestroyComponent _debug))))))

(event EventTick
  (params (DeltaSeconds :type Float%20%28single-precision%29))
  (bind _healthwidget (Variables|Default|GetHealthWidget))
  ;[1 1 1] Update UI Tick
  (Class|SATORIAICharacter|HealthBarProjection _healthwidget 2048.0 0.1 0.5)
  (bind _aswp_enemy_life_bar (Utilities|Casting|CastToWP_EnemyLifeBar (UserInterface|GetWidget _healthwidget)))
  (Class|SATORIEnemyHealthBar|UpdateHealthBar _aswp_enemy_life_bar (stale UpdateHealthBarPercent(EnemyStatComponent) Health) (stale UpdateHealthBarPercent(EnemyStatComponent) MaxHealth)))

(fn ConstructionScript)