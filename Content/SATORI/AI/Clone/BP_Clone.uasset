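; BP_Clone is a timed clone that lures AI characters and destroys itself when its lifetime expires.
; BeginPlay starts the death timer and initializes a widget timer, which Tick updates and turns toward the camera.
; On death it removes a gameplay tag from each lured SATORI_AICharacter.
; ChangeMaterial plays a color timeline forward or backward to tint two dynamic materials, but their creation nodes are never executed.
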(event Custom|ChangeMaterial
  (params (RateChange :type Float%20%28single-precision%29) (Dir :type Boolean))
  (Components|Timeline|SetPlayRate (Variables|Default|GetColorChange) (/ 1.0 RateChange))
  (if Dir
    (bind _color (Timeline|ColorChange PlayFromStart)
      (:Update
        (Rendering|Material|SetVectorParameterValue (Variables|Default|GetDynamicMaterial0) "ColorChange" (Math|Conversions|ToLinearColor(Vector) _color) :!class /Script/Engine.MaterialInstanceDynamic)
        (Rendering|Material|SetVectorParameterValue (Variables|Default|GetDynamicMaterial1) "ColorChange" (Math|Conversions|ToLinearColor(Vector) _color) :!class /Script/Engine.MaterialInstanceDynamic)))
    (else
      (Timeline|ColorChange ReverseFromEnd))))

(event Custom|Die
  (bind _returnvalue (Class|SATORICloneCharacter|GetArrayLured))
  (for _array_element _returnvalue
    (Utilities|IsValid _array_element
      (:Is%20Valid
        (bind _assatori_aicharacter (Utilities|Casting|CastToSATORI_AICharacter _array_element))
        (Class|SATORICharacterBase|RemoveGameplayTag _assatori_aicharacter (Variables|Default|GetTag%20to%20Remove)))))
  (Actor|DestroyActor))

(event EventBeginPlay
  (bind _clonemaxlife (Variables|Default|GetCloneMaxLife))
  (Utilities|FlowControl|Sequence
    (:then_1
      (bind _aswbp_clone_timer (Utilities|Casting|CastToWBP_CloneTimer (UserInterface|GetWidget (Variables|Default|GetTimer))))
      (bind _output_get (Variables|Default|SetAs%20WBP%20Clone%20Timer _aswbp_clone_timer))
      (Default|InitCloneLife _output_get _clonemaxlife)
      (Utilities|Time|SetTimerbyEvent (delegate Custom|Die) _clonemaxlife))))

(event EventTick
  (params (DeltaSeconds :type Float%20%28single-precision%29))
  (bind _timer (Variables|Default|GetTimer))
  (bind _output_get (Variables|Default|SetTimeAlive (+ DeltaSeconds (Variables|Default|GetTimeAlive))))
  (Default|UpdateTimeAlive (Variables|Default|GetAs%20WBP%20Clone%20Timer) _output_get)
  (Transformation|SetWorldRotation _timer (Math|Rotator|FindLookatRotation (Transformation|GetWorldLocation _timer) (Camera|GetCameraLocation (Game|GetPlayerCameraManager 0))) false false))

(fn ConstructionScript)