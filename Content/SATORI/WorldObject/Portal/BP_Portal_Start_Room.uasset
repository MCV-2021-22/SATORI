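; BP_Portal_Start_Room is a portal world object, named for the start room, that adds a gameplay tag to the player character.
; BeginPlay runs the parent logic, then caches the world location of the particle spawn component.
; PlayAnimationandEffectsPortal casts the first player pawn to SATORI_Character and applies TagToAdd, with no animation or effect calls of its own.
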(event EventBeginPlay
  (|CallParentFunction)
  (Variables|Default|SetSpawnParticleLocation (Transformation|GetWorldLocation (Variables|Default|GetSpawnParticleComponent))))

(event Collision|EventActorBeginOverlap
  (params (OtherActor :type Actor%20Object%20Reference))
  (|CallParentFunction OtherActor) ; This node is disabled and will not be called.\nDrag off pins to build functionality.
)

(event EventTick
  (params (DeltaSeconds :type Float%20%28single-precision%29))
  (|CallParentFunction DeltaSeconds) ; This node is disabled and will not be called.\nDrag off pins to build functionality.
)

(event EventPlayAnimationandEffectsPortal
  (bind _assatori_character (Utilities|Casting|CastToSATORI_Character (Game|Player|GetPlayerPawn 0)))
  (Class|SATORICharacterBase|AddGameplayTag _assatori_character (Variables|Default|GetTag%20to%20Add)))

(fn ConstructionScript
  (|CallParentFunction))