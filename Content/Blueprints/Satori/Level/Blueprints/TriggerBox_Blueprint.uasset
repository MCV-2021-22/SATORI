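; TriggerBox_Blueprint is a level transition trigger that carries player state out of the current level.
; When a ThirdPersonCharacter_prov overlaps its collision component, it copies the character's life, mana and ability number into SATORI_GameInstance so they persist across the load.
; It then calls OpenLevelByName on ThirdPersonGameMode, leaving the level change to the game mode.
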(event OnComponentBeginOverlap(CollisionComponent)
  (params (OverlappedComponent :type Primitive%20Component%20Object%20Reference) (OtherActor :type Actor%20Object%20Reference) (OtherComp :type Primitive%20Component%20Object%20Reference) (OtherBodyIndex :type Integer) (bFromSweep :type Boolean) (SweepResult :type Hit%20Result%20Structure%20%28by%20ref%29))
  (bind _asthird_person_character_prov (Utilities|Casting|CastToThirdPersonCharacter_prov OtherActor))
  (bind _assatori_game_instance (Utilities|Casting|CastToSATORI_GameInstance (Game|GetGameInstance)))
  (Variables|/Script/SATORI.SATORI_GameInstance|SetPlayerLife _assatori_game_instance (Variables|/Game/Blueprints/Player/Blueprints/ThirdPersonCharacter_prov.ThirdPersonCharacter_prov_C|GetPlayerLife _asthird_person_character_prov))
  (Variables|/Script/SATORI.SATORI_GameInstance|SetPlayerMana _assatori_game_instance (Variables|/Game/Blueprints/Player/Blueprints/ThirdPersonCharacter_prov.ThirdPersonCharacter_prov_C|GetPlayerMana _asthird_person_character_prov))
  (Variables|/Script/SATORI.SATORI_GameInstance|SetPlayerAbility _assatori_game_instance (Variables|/Game/Blueprints/Player/Blueprints/ThirdPersonCharacter_prov.ThirdPersonCharacter_prov_C|GetAbilityNumber _asthird_person_character_prov))
  (bind _asthird_person_game_mode (Utilities|Casting|CastToThirdPersonGameMode (Game|GetGameMode)))
  (Default|OpenLevel _asthird_person_game_mode))

(event EventBeginPlay)

(event EventTick
  (params (DeltaSeconds :type Float%20%28single-precision%29)))

(fn ConstructionScript)