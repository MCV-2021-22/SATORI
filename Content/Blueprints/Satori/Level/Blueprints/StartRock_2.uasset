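; StartRock_2 is an interactable level actor that loads the "Sala1" level when the player presses Interact beside it.
; Overlap of either prototype third-person character with its Box shows an Ekey prompt widget and opens a Gate, and leaving reverses both.
; Interact briefly flags the prompt as pressed, then passes through the Gate to destroy the Box, disable interaction and open the level.
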(event OnComponentBeginOverlap(Box)
  (params (OverlappedComponent :type Primitive%20Component%20Object%20Reference) (OtherActor :type Actor%20Object%20Reference) (OtherComp :type Primitive%20Component%20Object%20Reference) (OtherBodyIndex :type Integer) (bFromSweep :type Boolean) (SweepResult :type Hit%20Result%20Structure%20%28by%20ref%29))
  (Utilities|Casting|CastToThirdPersonCharacter_prov OtherActor
    (:then
      _)
    (:CastFailed
      (Utilities|Casting|CastToThirdPersonCharacter_prov_2 OtherActor)))
  (bind _returnvalue (UserInterface|CreateWidget "/Game/Blueprints/Satori/Level/Blueprints/Ekey.Ekey_C"))
  (UserInterface|Viewport|AddtoViewport _returnvalue 0)
  (Utilities|FlowControl|Gate true) ; enters at Open
)

(event OnComponentEndOverlap(Box)
  (params (OverlappedComponent :type Primitive%20Component%20Object%20Reference) (OtherActor :type Actor%20Object%20Reference) (OtherComp :type Primitive%20Component%20Object%20Reference) (OtherBodyIndex :type Integer))
  (Utilities|Casting|CastToThirdPersonCharacter_prov OtherActor
    (:then
      _)
    (:CastFailed
      (Utilities|Casting|CastToThirdPersonCharacter_prov_2 OtherActor)))
  (Widget|RemovefromParent (stale OnComponentBeginOverlap(Box) _returnvalue))
  (Utilities|FlowControl|Gate true) ; enters at Close
)

(event EventBeginPlay
  (Input|EnableInput (Game|GetPlayerController 0))
  (Variables|Default|SetcanInteract true))

(event Collision|EventActorBeginOverlap
  (params (OtherActor :type Actor%20Object%20Reference)))

(event EventTick
  (params (DeltaSeconds :type Float%20%28single-precision%29)))

(event Input|ActionEvents|InputActionInteract
  (params (Key :type Key%20Structure :default "None"))
  (:Pressed
    (if (Variables|Default|GetcanInteract)
      (Variables|/Game/Blueprints/Satori/Level/Blueprints/Ekey.Ekey_C|SetisPressed (stale OnComponentBeginOverlap(Box) _returnvalue) true)
      (Utilities|FlowControl|Delay 0.2)
      (Variables|/Game/Blueprints/Satori/Level/Blueprints/Ekey.Ekey_C|SetisPressed (stale OnComponentBeginOverlap(Box) _returnvalue) false)
      (Utilities|FlowControl|Gate true
        (:Exit
          (Utilities|Casting|CastToThirdPersonGameMode (Game|GetGameMode))
          (Components|DestroyComponent (Variables|Default|GetBox))
          (Variables|Default|SetcanInteract false)
          (Game|OpenLevel(byName) "Sala1"))))))

(fn ConstructionScript)